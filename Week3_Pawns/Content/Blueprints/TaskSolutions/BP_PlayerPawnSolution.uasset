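; Tutorial solution pawn showing two ways to move a Pawn without a CharacterMovementComponent.
; MovementTypeOne feeds forward/right axes, scaled by MoveSpeed and delta time, into AddMovementInput, applying the consumed vector to the capsule.
; MovementTypeTwo offsets the actor directly along world X/Y using the same scaling.
; Tick is empty; both movement calls and the debug toggle of UseMovementTypeOne are unconnected.
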(event EventTick
  (params (DeltaSeconds :type Float%20%28single-precision%29)))

(event Input|KeyboardEvents|T
  (params (Key :type Key%20Structure :default "None"))
  ;[0 0 0] DEBUG LOGIC --- Usually don't assign specific key bindings in the EventGraph, use ProjectSettings->Input for more control. For Debug it's kinda ok.
)

(fn ConstructionScript)

(fn MovementTypeOne
  (Utilities|FlowControl|Sequence
    (:then_0
      ;[0 0 0] Because the Pawn doesn't have a CharacterMovementComponent the AddMovementInput is NOT automatically tracked and calculated, so we need to do that here, constantly recording it with ConsumeMovementInputVector and then applying an Offset to our world location.
      (bind _returnvalue (Class|Pawn|ConsumeMovementInputVector))
      (Transformation|AddWorldOffset (Variables|Default|GetCapsule) _returnvalue false false))
    (:then_1
      ;[0 0 0] MovementInput can be taken here rather than the MoveForward and MoveRight Axis as they're essentially running a tick event. Not we just use the Axis values below in the Scale Value
      (Pawn|Input|AddMovementInput (Transformation|GetActorForwardVector) (* (Input|AxisValues|GetMoveForward) (* (Variables|Default|GetMoveSpeed) (Utilities|Time|GetWorldDeltaSeconds))) false))
    (:then_2
      (Pawn|Input|AddMovementInput (Transformation|GetActorRightVector) (* (Input|AxisValues|GetMoveRight) (* (Variables|Default|GetMoveSpeed) (Utilities|Time|GetWorldDeltaSeconds))) false))))

(fn MovementTypeTwo
  ;[0 0 0] A VERY simplified version of what's happening in the CharacterMovementComponent. Adding an offset to the current world location based on the inputs being pressed and the speeds being assigned. This is not using any of the ConsumeInput functionality so it's a basic form of the most manual way we can add movement to a default pawn
  (Transformation|AddActorWorldOffset (Math|Vector|MakeVector (* (Input|AxisValues|GetMoveForward) (* (Variables|Default|GetMoveSpeed) (Utilities|Time|GetWorldDeltaSeconds))) (* (Input|AxisValues|GetMoveRight) (* (Variables|Default|GetMoveSpeed) (Utilities|Time|GetWorldDeltaSeconds))) 0.0)))